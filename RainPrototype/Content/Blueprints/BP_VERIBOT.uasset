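; VERIBOT enemy that chases the player on sight, kills them on hit, and returns to its spawn point.
; A detection sphere flags the player in range, and Tick line-traces to update the last-seen target and drive Idle, Chasing and Returning states.
; Movement teleports a fixed step per frame without sweep, using a clamped vector inverse lerp to avoid overshoot.
; Debug spheres, traces and prints are left active.
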(event `self.ReceiveBeginPlay`
  (bind _skeletalmeshcomponent (`self.SkeletalMeshComponent`))
  (bind _output_get (set `self.Home` (`SceneComponent.K2_GetComponentLocation` _skeletalmeshcomponent)))
  (set `self.Target` _output_get)
  (set `self.Initial Rotation` (`SceneComponent.K2_GetComponentRotation` _skeletalmeshcomponent)))

(event `self.ReceiveHit`
  (params (MyComp :type "PrimitiveComponent Object Reference") (Other :type "Actor Object Reference") (OtherComp :type "PrimitiveComponent Object Reference") (bSelfMoved :type Boolean) (HitLocation :type "Vector Structure") (HitNormal :type "Vector Structure") (NormalImpulse :type "Vector Structure") (Hit :type "HitResult Structure (by ref)"))
  (bind (_player _cached_or_cast_success _presumed_player_was_player) (`self.Lazy Instantiate CachedPlayer` Other))
  (if (and _cached_or_cast_success _presumed_player_was_player)
    (`/Game/ThirdPersonBP/Blueprints/ThirdPersonCharacter.Die` _player)
    ;[1 1 1 1 12] If the player was hit, even if the target hasn't technically been reached yet, set target to current position to stop chasing
    (set `self.Target` (`SceneComponent.K2_GetComponentLocation` (`self.SkeletalMeshComponent`)))))

(event `self.DetectZone.OnComponentBeginOverlap`
  (params (OverlappedComponent :type "PrimitiveComponent Object Reference") (OtherActor :type "Actor Object Reference") (OtherComp :type "PrimitiveComponent Object Reference") (OtherBodyIndex :type Integer) (bFromSweep :type Boolean) (SweepResult :type "HitResult Structure (by ref)"))
  (`self.Update Player in Range` OtherActor true)
  (`KismetSystemLibrary.PrintString` "Player in range"))

(event `self.DetectZone.OnComponentEndOverlap`
  (params (OverlappedComponent :type "PrimitiveComponent Object Reference") (OtherActor :type "Actor Object Reference") (OtherComp :type "PrimitiveComponent Object Reference") (OtherBodyIndex :type Integer))
  (`self.Update Player in Range` OtherActor)
  (`KismetSystemLibrary.PrintString` "Player out of range"))

(event `self.ReceiveTick`
  (params (DeltaSeconds :type "Float (single-precision)"))
  (bind _detectzone (`self.DetectZone`))
  (bind _skeletalmeshcomponent (`self.SkeletalMeshComponent`))
  (bind _cachedplayer (`self.CachedPlayer`))
  (bind _state (`self.State`))
  (bind _skeletalmeshcomponent_2 (`self.SkeletalMeshComponent`))
  (bind _returnvalue (`self.K2_GetActorLocation` _cachedplayer))
  (bind _returnvalue_2 (`SceneComponent.K2_GetComponentLocation` _detectzone))
  (bind _returnvalue_3 (`SceneComponent.K2_GetComponentLocation` _skeletalmeshcomponent_2))
  (bind _returnvalue_4 (`|EnumEquality` _state "NewEnumerator1"))
  (bind _returnvalue_5 (`KismetMathLibrary.SelectVector` (`self.Home`) (`self.Target`) _returnvalue_4))
  (`KismetSystemLibrary.DrawDebugSphere` _returnvalue_2 (`SphereComponent.GetScaledSphereRadius` _detectzone))
  (`KismetSystemLibrary.DrawDebugSphere` _returnvalue_2 5.0 12 (struct :`R` 1.0 :`A` 1.0))
  (`KismetSystemLibrary.PrintString` (`KismetStringLibrary.Concat_StrStr` "Enemy State: " (`|GetEnumeratorNameAsString` (`self.State`))) true true (struct :`R` 1.0 :`G` 0.369792 :`B` 0.369792 :`A` 1.0) 0.0)
  (switch `/Game/Blueprints/EnemyState` _state
    (:`NewEnumerator0`
      ;[1 1 1] Start rotating back to default rotation
      (`SceneComponent.K2_SetWorldRotation` _skeletalmeshcomponent (`KismetMathLibrary.RInterpTo` (`SceneComponent.K2_GetComponentRotation` _skeletalmeshcomponent) (`self.Initial Rotation`) DeltaSeconds (`self.Move Speed`)) false false))
    (:`NewEnumerator1`
      ;[1 1 1] If returning/chasing, move towards home/target respectively
      (`self.No Overshoot Move To` _skeletalmeshcomponent_2 DeltaSeconds _returnvalue_3 _returnvalue_5 :!label _label)
      ;[1 1 1] If reached destination (home/target), set state accordingly
      (if (== _returnvalue_3 _returnvalue_5 :`ErrorTolerance` 0.1)
        (bind _output_get (set `self.State` (select `bool` _returnvalue_4 :`false` "NewEnumerator1" :`true` "NewEnumerator0" :!type "/Game/Blueprints/EnemyState Enum")))
        (`KismetSystemLibrary.PrintString` "set state to returning or idle")))
    (:`NewEnumerator2`
      (goto _label)))
  ;[1 1 1] If the player is in range or this enemy is already chasing them, raycast in their direction.
  (if (or (`self.Player in Range`) (`|EnumEquality` _output_get "NewEnumerator2"))
    (if (`KismetSystemLibrary.IsValid` _cachedplayer)
      (bind (_outhit _returnvalue_6) (`KismetSystemLibrary.LineTraceSingleForObjects` (`SceneComponent.K2_GetComponentLocation` (`self.SkeletalMeshComponent`)) _returnvalue (`|MakeArray` "ObjectTypeQuery1" "ObjectTypeQuery2" "ObjectTypeQuery4" "ObjectTypeQuery5" "ObjectTypeQuery6" :!type "EObjectTypeQuery Enum") false (`|MakeArray` _cachedplayer :!type "Actor Object Reference") "ForOneFrame"))
      ;[1 1 1] If nothing was hit, the enemy has line of sight to the player; set target to their current position and give chase.
      (if (not _returnvalue_6)
        (set `self.Target` _returnvalue)
        (set `self.State` "NewEnumerator2")))))

(fn `Get Target or Home`
  (params (Chasing :type Boolean))
  (returns (`Home or Target` :type "Vector Structure"))
  (if Chasing
    (return (`self.Target`))
    (else
      (return (`self.Home`)))))

(fn `Inverse Lerp Vector3`
  (params (from :type "Vector Structure") (to :type "Vector Structure") (value :type "Vector Structure"))
  (returns (t :type "Float (double-precision)"))
  (bind _returnvalue (- to from))
  ;[1 1 1 1 16] Math from: https://answers.unity.com/questions/1271974/inverselerp-for-vector3.html#answer-1274648
  (return (`KismetMathLibrary.FClamp` (/ (`KismetMathLibrary.Dot_VectorVector` (- value from) _returnvalue) (`KismetMathLibrary.Dot_VectorVector` _returnvalue _returnvalue)))))

(fn `Lazy Instantiate CachedPlayer`
  (params (`Presumed Player` :type "Actor Object Reference"))
  (returns (Player :type "/Game/ThirdPersonBP/Blueprints/ThirdPersonCharacter Object Reference") (`Cached or Cast Success` :type Boolean) (`Presumed Player Was Player` :type Boolean))
  (bind _cachedplayer (`self.CachedPlayer`))
  (if (`KismetSystemLibrary.IsValid` _cachedplayer)
    (return _cachedplayer true (== _cachedplayer `Presumed Player`))
    (else
      (bind _asthird_person_character (cast `/Game/ThirdPersonBP/Blueprints/ThirdPersonCharacter` `Presumed Player`)
        (:`then`
          (bind _output_get (set `self.CachedPlayer` _asthird_person_character))
          (return _output_get true true))
        (:`CastFailed`
          (return _asthird_person_character false false))))))

(fn `No Overshoot Move To`
  (params (`Thing to Move` :type "SceneComponent Object Reference") (`Delta Time` :type "Float (double-precision)") (`Current Location` :type "Vector Structure") (`Target Location` :type "Vector Structure"))
  (bind _returnvalue (`KismetMathLibrary.FindLookAtRotation` `Current Location` `Target Location`))
  (bind _returnvalue_2 (`|EnumInequality` (`self.State`) "NewEnumerator2"))
  (`KismetSystemLibrary.PrintString` (`KismetStringLibrary.Concat_StrStr` "Current = " (`KismetStringLibrary.Conv_VectorToString` `Current Location`) (`KismetMathLibrary.SelectString` " \nHome = " " \nTarget = " _returnvalue_2) (`KismetStringLibrary.Conv_VectorToString` `Target Location`)) true true (struct :`R` 1.0 :`G` 0.875039 :`A` 1.0) 0.0)
  (`SceneComponent.K2_SetWorldRotation` `Thing to Move` (`KismetMathLibrary.MakeRotator` (.roll (`KismetMathLibrary.SelectRotator` (`KismetMathLibrary.RInterpTo` (`SceneComponent.K2_GetComponentRotation` `Thing to Move`) _returnvalue `Delta Time` (`self.Move Speed`)) _returnvalue _returnvalue_2)) 0.0 (.yaw (`KismetMathLibrary.SelectRotator` (`KismetMathLibrary.RInterpTo` (`SceneComponent.K2_GetComponentRotation` `Thing to Move`) _returnvalue `Delta Time` (`self.Move Speed`)) _returnvalue _returnvalue_2))) false false)
  (bind _sweephitresult (`SceneComponent.K2_SetWorldLocation` `Thing to Move` (`KismetMathLibrary.VLerp` `Current Location` `Target Location` (`self.Inverse Lerp Vector3` `Current Location` `Target Location` (+ `Current Location` (* (`SceneComponent.GetForwardVector` `Thing to Move`) (`self.Move Speed`))))) false true))
  (bind (_bblockinghit _binitialoverlap _time _distance _location _impactpoint _normal _impactnormal _physmat _hitactor) (`GameplayStatics.BreakHitResult` _sweephitresult))
  (`KismetSystemLibrary.PrintString` (`KismetStringLibrary.Concat_StrStr` "Blocking Hit = " (`KismetStringLibrary.Conv_BoolToString` _bblockinghit) " \n" (`KismetSystemLibrary.GetDisplayName` _hitactor)) true true (struct :`R` 1.0 :`B` 0.866621 :`A` 1.0) 0.0)
  (return))

(fn `Update Player in Range`
  (params (`Overlap Other` :type "Actor Object Reference") (`Beginning Overlap` :type Boolean))
  (bind (_player _cached_or_cast_success _presumed_player_was_player) (`self.Lazy Instantiate CachedPlayer` `Overlap Other`))
  (if (and _cached_or_cast_success _presumed_player_was_player)
    (set `self.Player in Range` `Beginning Overlap`)))

(fn `UserConstructionScript`)